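; BP_Spawnable is a collectible, apparently a star, that serves as the player's current waypoint.
; On BeginPlay it registers itself with the player pawn through SetWaypoint and calls SendWaypointData.
; Each tick it rotates to face the player character's mesh.
; When the player overlaps its sphere, it resets the game mode's timer, asks BP_Spawner to spawn another star, and destroys itself.
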(event OnComponentBeginOverlap(Sphere)
  (params (OverlappedComponent :type Primitive%20Component%20Object%20Reference) (OtherActor :type Actor%20Object%20Reference) (OtherComp :type Primitive%20Component%20Object%20Reference) (OtherBodyIndex :type Integer) (bFromSweep :type Boolean) (SweepResult :type Hit%20Result%20Structure%20%28by%20ref%29))
  (if (== OtherActor (Game|Player|GetPlayerPawn 0))
    (bind _asbp_top_down_polaris (Utilities|Casting|CastToBP_TopDownPolaris (Game|GetGameMode)))
    (Default|ResetTimer _asbp_top_down_polaris)
    (bind _returnvalue (Actor|GetActorOfClass "/Game/GameMechanics/BP_Spawner.BP_Spawner_C"))
    (Default|SpawnStar _returnvalue)
    (Actor|DestroyActor)))

(event EventBeginPlay
  (bind _self self)
  (bind _asbp_top_down_polaris_char (Utilities|Casting|CastToBP_TopDownPolarisChar (Game|Player|GetPlayerPawn 0)))
  (Default|SetWaypoint _asbp_top_down_polaris_char _self)
  (Default|CallSendWaypointData _self))

(event Collision|EventActorBeginOverlap
  (params (OtherActor :type Actor%20Object%20Reference)))

(event EventTick
  (params (DeltaSeconds :type Float%20%28single-precision%29))
  (bind _asbp_top_down_character (Utilities|Casting|CastToBP_TopDownCharacter (Game|GetPlayerCharacter 0)))
  (Transformation|SetActorRotation (Math|Rotator|FindLookatRotation (Transformation|GetWorldLocation (Variables|Default|GetSphere1)) (Transformation|GetWorldLocation (Variables|/Script/Engine.Character|GetMesh _asbp_top_down_character)))))

(fn ConstructionScript)