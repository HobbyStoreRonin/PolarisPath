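; BP_Spawner sets up a randomly chosen mission and spawns its waypoint actors and exit.
; On BeginPlay it picks from Missions, passes the start position to the BP_TopDownPolaris game mode, then spawns the first "star" and BP_Exit.
; NextWaypoint spawns each following star from the mission's waypoint class and position, advancing an index until the list runs out.
; StartTimer is an empty stub.
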(event Custom|SpawnStar
  (bind _currentstar (Variables|Default|GetCurrentStar))
  (bind _mission (Variables|Default|GetMission))
  (bind _output (Utilities|Array|Get(acopy) (.waypoints _mission) _currentstar))
  (if (>= (- (Utilities|Array|Length (.waypoints _mission)) 1) _currentstar)
    (Game|SpawnActorfromClass (.tospawn _output) (.position _output) "AdjustIfPossibleButAlwaysSpawn" "MultiplyWithRoot" 0 0)
    (CallFunction|IncrementWaypoint)))

(event Custom|Start%20Timer)

(event Custom|IncrementWaypoint
  (bind _result (Math|Integer|IncrementInt (Variables|Default|GetCurrentStar))
    (:%20%20
      (Variables|Default|SetCurrentStar _result))))

(event Custom|GetNewMission
  (params (MissionNumber :type Integer))
  (Variables|Default|SetMission (Utilities|Array|Get(acopy) (.missions (Variables|Default|GetMissions)) MissionNumber)))

(event Custom|SpawnExit
  (Game|SpawnActorfromClass "/Game/GameMechanics/BP_Exit.BP_Exit_C" (.endposition (Variables|Default|GetMission)) "AdjustIfPossibleButAlwaysSpawn" "MultiplyWithRoot" 0 0))

(event EventBeginPlay
  (CallFunction|GetNewMission (.OutIndex (Utilities|Array|Random (Utilities|Struct|BreakST_Missions (Variables|Default|GetMissions)))))
  (bind _asbp_top_down_polaris (Utilities|Casting|CastToBP_TopDownPolaris (Game|GetGameMode)))
  (Default|SetStartLocation _asbp_top_down_polaris (.startposition (Variables|Default|GetMission)))
  (CallFunction|SpawnStar)
  (CallFunction|SpawnExit)
  (CallFunction|StartTimer))

(event Collision|EventActorBeginOverlap
  (params (OtherActor :type Actor%20Object%20Reference)))

(event EventTick
  (params (DeltaSeconds :type Float%20%28single-precision%29)))

(fn ConstructionScript)

(fn NextWaypoint
  (CallFunction|SpawnStar))